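; BP_EnnemiParent is a base enemy that chases the first-person player and triggers game over on reaching them.
; BeginPlay caches the player character and game mode.
; ChasePP runs AIMoveTo on the player, retrying on failure; on success it zeroes the player's walk speed and plays the LoseGame animation on the game mode's widget.
; ActiveEnnemie is an empty event, and nothing here calls ChasePP.
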(event Custom|ActiveEnnemie)

(event Custom|ChasePP
  (bind _gm (Variables|Default|GetGM))
  (bind _wbpgame (Variables|/Game/FirstPerson/Blueprints/BP_FirstPersonGameMode.BP_FirstPersonGameMode_C|GetWBPGame _gm))
  (AI|AIMoveTo self "0, 0, 0" (Variables|Default|GetPP) 5.0 false
    (:OnSuccess
      (Variables|/Script/Engine.CharacterMovementComponent|SetMaxWalkSpeed (Variables|/Script/Engine.Character|GetCharacterMovement (Variables|Default|GetPP)) 0.0)
      (UserInterface|Animation|PlayAnimation _wbpgame (Variables|/Game/UI/WBP_Game.WBP_Game_C|GetLoseGame _wbpgame) 0.0 1 "Forward" 1.0 false))
    (:OnFail
      (CallFunction|ChasePP))))

(event EventBeginPlay
  (bind _asbp_first_person_character (Utilities|Casting|CastToBP_FirstPersonCharacter (Game|GetPlayerCharacter 0)))
  (Variables|Default|SetPP _asbp_first_person_character)
  (bind _asbp_first_person_game_mode (Utilities|Casting|CastToBP_FirstPersonGameMode (Game|GetGameMode)))
  (Variables|Default|SetGM _asbp_first_person_game_mode))

(fn ConstructionScript)