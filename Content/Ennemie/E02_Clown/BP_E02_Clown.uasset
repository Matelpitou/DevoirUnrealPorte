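; BP_E02_Clown is the Clown enemy Blueprint, extending a parent enemy's BeginPlay and activation events.
; Its spotlight stays hidden in game until ActiveEnnemie reveals it and calls ChasePP.
; Activation also plays a speed timeline, scaled by RateSpeed, whose Alpha multiplies MWS to drive the character's max walk speed over time.
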(event EventBeginPlay
  (|CallParentFunction)
  (Development|SetHiddeninGame (Variables|Default|GetSpotLight) true false))

(event EventActiveEnnemie
  (|CallParentFunction)
  (Utilities|FlowControl|Sequence
    (:then_0
      (Components|Timeline|SetPlayRate (Variables|Default|GetTL_Speed) (/ 1.0 (Variables|Default|GetRateSpeed)))
      (bind _alpha (Timeline|TL_Speed PlayFromStart)
        (:Update
          (Variables|/Script/Engine.CharacterMovementComponent|SetMaxWalkSpeed (Variables|Character|GetCharacterMovement) (* _alpha (Variables|Default|GetMWS))))))
    (:then_1
      (Development|SetHiddeninGame (Variables|Default|GetSpotLight) false false)
      (CallFunction|ChasePP))))

(fn ConstructionScript)