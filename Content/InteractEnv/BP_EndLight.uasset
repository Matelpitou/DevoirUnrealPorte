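; BP_EndLight is an end-sequence spotlight actor that starts hidden and fires once, when Activate finds at least three linked doors closed.
; It then reveals the spotlight, initializes and activates the end door, calls ActiveLight(false) on linked lights, and activates linked enemies after a short delay.
; FixPlayer re-calls itself on a short delay to keep the actor rotated toward the player.
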(event Custom|FixPlayer
  ;[1 1 1] Intéraction des portes
  ;;[1 1 1] S'oriente en fonction du player
  (Transformation|SetActorRotation (Math|Rotator|FindLookatRotation (Transformation|GetActorLocation) (Transformation|GetActorLocation (Variables|Default|GetPP))))
  (Utilities|FlowControl|Delay 0.05)
  (CallFunction|FixPlayer))

(event EventBeginPlay
  ;[1 1 1] Start
  (Development|SetHiddeninGame (Variables|Default|GetSpotLight) true false)
  (bind _asbp_first_person_character (Utilities|Casting|CastToBP_FirstPersonCharacter (Game|GetPlayerCharacter 0)))
  (Variables|Default|SetPP _asbp_first_person_character))

(event EventActivate
  (bind _bp_enddoor (Variables|Default|GetBP_EndDoor))
  ;[1 1 1] Intéraction des portes
  ;;[1 1 1] Check si les 3 portes sont fermés
  (Variables|Default|SetInt 0)
  (for _array_element (Variables|Default|GetDoor)
    (if (not (Variables|/Game/InteractEnv/BP_Porte.BP_Porte_C|GetDoorOpen? _array_element))
      (bind _result (Math|Integer|IncrementInt (Variables|Default|GetInt))
        (:%20%20
          (Variables|Default|SetInt _result)))))
  ;;[1 1 1] Si les 3 portes sont bien fermés
  (if (>= (Variables|Default|GetInt) 3)
    (Utilities|FlowControl|DoOnce false
      (:Completed
        ;;[1 1 1] Désactive les portes et actives la light
        (Development|SetHiddeninGame (Variables|Default|GetSpotLight) false false)
        (CallFunction|FixPlayer)
        (Default|InitialDoor _bp_enddoor)
        (Default|ActivateDoor _bp_enddoor)
        (for _array_element_2 (Variables|Default|GetBP_Light)
          (Default|ActiveLight _array_element_2 false))
        ;;[1 1 1] Active les ennemis
        (Utilities|FlowControl|Delay 0.75)
        (for _array_element_3 (Variables|Default|GetBP_Ennemie)
          (Default|ActiveEnnemie _array_element_3))))))

(fn ConstructionScript)