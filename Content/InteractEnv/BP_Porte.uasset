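; BP_Porte is a toggleable door that swings by yaw between its initial rotation and a configurable maximum angle.
; BeginPlay caches both rotations, scales timeline speed from SpeedTurnDoor, hides the spotlight and applies StartOpen through ActivateDoor.
; ActivateDoor flips DoorOpen, plays or reverses the rotation timeline, and colors the spotlight red when opening, green when closing.
; The timeline update forces white for LastDoor; InitialDoor reveals the spotlight.
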(event Custom|ActivateDoor
  ;[1 1 1] Active les portes
  (if (Variables|Default|GetDoorOpen?)
    (Variables|Default|SetDoorOpen? false)
    (CallFunction|ColorSpot (Variables|Default|GetGreen))
    (bind _alpha (Timeline|TL_RotateDoor Reverse)
      (:Update
        (Transformation|SetRelativeRotation (Variables|Default|GetSphere) (Math|Rotator|Lerp(Rotator) (Variables|Default|GetRotInit) (Variables|Default|GetRotEnd) _alpha) false false)
        ;;[1 1 1] Override blanc pour la derniere porte
        (if (Variables|Default|GetLastDoor?)
          (CallFunction|ColorSpot "(R=1.000000,G=1.000000,B=1.000000,A=1.000000)"))))
    (else
      (Variables|Default|SetDoorOpen? true)
      (CallFunction|ColorSpot (Variables|Default|GetRed))
      (Timeline|TL_RotateDoor Play))))

(event Custom|InitialDoor
  (Development|SetHiddeninGame (Variables|Default|GetSpotLight) false false))

(event EventBeginPlay
  (bind _sphere (Variables|Default|GetSphere))
  (bind _relativerotation (Variables|/Script/Engine.SceneComponent|GetRelativeRotation _sphere))
  (Components|Timeline|SetPlayRate (Variables|Default|GetTL_RotateDoor) (/ 1.0 (Variables|Default|GetSpeedTurnDoor)))
  (Variables|Default|SetRotInit (Variables|/Script/Engine.SceneComponent|GetRelativeRotation (Variables|Default|GetSphere)))
  (Variables|Default|SetRotEnd (Math|Rotator|MakeRotator (.roll _relativerotation) (.pitch _relativerotation) (+ (.yaw _relativerotation) (Variables|Default|GetAngleMaxDoor))))
  (Development|SetHiddeninGame (Variables|Default|GetSpotLight) true false)
  (if (Variables|Default|GetStartOpen?)
    (Variables|Default|SetDoorOpen? false)
    (CallFunction|ActivateDoor)
    (else
      (Variables|Default|SetDoorOpen? true)
      (CallFunction|ActivateDoor))))

(fn ConstructionScript)

(fn ColorSpot
  (params (Color :type Linear%20Color%20Structure))
  (Rendering|Components|Light|SetLightColor (Variables|Default|GetSpotLight) Color true))