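; Interactable candle Blueprint whose flame visibility at BeginPlay follows its Active flag.
; Activate switches on NameBougie: the main candle hides its point light and flame, then calls CanActivateEvent on every linked light wall in BPLightWall.
; InRange defers to the parent class and adds no behavior of its own.
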(event EventBeginPlay
  (if (Variables|Default|GetActive?)
    (Development|SetHiddeninGame (Variables|Default|GetCandle_Flame) false false)
    (else
      (Development|SetHiddeninGame (Variables|Default|GetCandle_Flame) true false))))

(event EventInRange
  (params (Activable? :type Boolean))
  (|CallParentFunction false)
  (if Activable?
    _))

(event EventActivate
  (switch name (Variables|Default|GetNameBougie)
    (:MainBougie
      (Development|SetHiddeninGame (Variables|Default|GetPointLight) true false)
      (Development|SetHiddeninGame (Variables|Default|GetCandle_Flame) true false)
      (for _array_element (Variables|Default|GetBP_LightWall)
        (Default|CanActivateEvent _array_element)))))

(fn ConstructionScript)